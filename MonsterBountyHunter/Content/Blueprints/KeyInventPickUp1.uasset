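; Key pickup actor that places item ID 1 into the player's five-slot inventory.
; On actor overlap, if CanPickUp is set, it casts the player character to TorchController and fills the first slot holding 0, then destroys itself.
; If all five slots are taken, it prints that the inventory is full.
; The overlapping actor is never checked, and BeginPlay only runs a short delay with nothing after it.
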(event `self.ReceiveBeginPlay`
  (`KismetSystemLibrary.Delay` 0.2))

(event `self.ReceiveActorBeginOverlap`
  (params (OtherActor :type "Actor Object Reference"))
  (if (`self.CanPickUp`)
    (bind _astorch_controller (cast `/Game/Blueprints/TorchController` (`GameplayStatics.GetPlayerCharacter` 0)))
    (if (== (`/Game/Blueprints/TorchController.Slot1Item` _astorch_controller) 0)
      (set `/Game/Blueprints/TorchController.Slot1Item` 1 _astorch_controller)
      (`self.K2_DestroyActor`)
      (elif (== (`/Game/Blueprints/TorchController.Slot2Item` _astorch_controller) 0)
        (set `/Game/Blueprints/TorchController.Slot2Item` 1 _astorch_controller)
        (`self.K2_DestroyActor`)
        (elif (== (`/Game/Blueprints/TorchController.Slot3Item` _astorch_controller) 0)
          (set `/Game/Blueprints/TorchController.Slot3Item` 1 _astorch_controller)
          (`self.K2_DestroyActor`)
          (elif (== (`/Game/Blueprints/TorchController.Slot4Item` _astorch_controller) 0)
            (set `/Game/Blueprints/TorchController.Slot4Item` 1 _astorch_controller)
            (`self.K2_DestroyActor`)
            (elif (== (`/Game/Blueprints/TorchController.Slot5Item` _astorch_controller) 0)
              (set `/Game/Blueprints/TorchController.Slot5Item` 1 _astorch_controller)
              (`self.K2_DestroyActor`)
              (else
                (`KismetSystemLibrary.PrintString` "Inventory is full")))))))))

(fn `UserConstructionScript`)