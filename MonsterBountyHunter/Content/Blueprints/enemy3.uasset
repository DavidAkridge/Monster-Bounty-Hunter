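; Enemy that turns to face a TorchController pawn seen through PawnSensing and fires at it.
; Shots spawn another TorchController at the projectile spawn point and launch its mesh along the Cube's forward vector, gated by a short boolean-and-delay cooldown.
; BeginPlay stores three patrol positions and picks a random index, but the timeline meant to move it never runs and its lerp is unconnected.
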(event `self.ReceiveBeginPlay`
  ;[1 1 1] SetThePetrolPoints
  (set `self.Patrolpoints` (`|MakeArray` (`SceneComponent.K2_GetComponentLocation` (`self.MovePosition1`)) (`SceneComponent.K2_GetComponentLocation` (`self.MovePosition2`)) (`SceneComponent.K2_GetComponentLocation` (`self.MovePosition3`))))
  (`self.GetRandomLocation`))

(event `self.PawnSensing.OnSeePawn`
  (params (Pawn :type "Pawn Object Reference"))
  ;[1 1 1] LookAtAndShootPawn
  (bind _astorch_controller (cast `/Game/Blueprints/TorchController` Pawn))
  (`|ExecutionSequence`
    (:`then_0`
      (`self.K2_SetActorRotation` (`KismetMathLibrary.FindLookAtRotation` (`self.K2_GetActorLocation`) (`self.K2_GetActorLocation` _astorch_controller))))
    (:`then_1`
      (if (`self.SpawnProjectile`)
        (bind _returnvalue (`|SpawnActorFromClass` "/Game/Blueprints/TorchController.TorchController_C" (`SceneComponent.K2_GetComponentToWorld` (`self.ProjectileSpawnLocation`)) "Undefined" "OverrideRootScale" null null))
        (`PrimitiveComponent.AddImpulse` (`Character.Mesh` _returnvalue) (* (`SceneComponent.GetForwardVector` (`self.Cube`)) (`self.ShootAmount`)) "None" true)
        (set `self.SpawnProjectile` false)
        (`KismetSystemLibrary.Delay` 0.2)
        (set `self.SpawnProjectile` true)))))

(fn `GetRandomLocation`
  (set `self.CurrentPetrolPoints` (`KismetMathLibrary.RandomInteger` (`KismetArrayLibrary.Array_Length` (`self.Patrolpoints`)))))

(fn `UserConstructionScript`)