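; Boss enemy AI that roams the navmesh, chases the player when Pawn Sensing sees a pawn, and attacks on contact.
; Roam and Chase set walk speed and use AIMoveTo toward random points or the player's location.
; HitBox overlap with a TorchController halts movement, applies delayed damage if still overlapping, then resumes chasing.
; AnyDamage lowers Health, Tick destroys the boss at zero, and InteractableArea overlaps toggle its input.
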(event `self.ReceiveBeginPlay`
  (`self.Roam`))

(event `Chase`
  ;[1 1 1] Enemy Stalking Player
  (set `CharacterMovementComponent.MaxWalkSpeed` 450.0 (`self.CharacterMovement`))
  (`|AIMoveTo` self (`self.K2_GetActorLocation` (`GameplayStatics.GetPlayerCharacter` 0))
    (:`OnSuccess`
      (`KismetSystemLibrary.Delay` 1.0)
      (`self.Roam`))))

(event `Roam`
  ;[1 1 1] Roaming
  (`KismetSystemLibrary.Delay` 5.0)
  (set `CharacterMovementComponent.MaxWalkSpeed` 200.0 (`self.CharacterMovement`))
  (`|AIMoveTo` self (`NavigationSystem.K2_GetRandomLocationInNavigableRadius` (`self.K2_GetActorLocation`) 1000.0)
    (:`then`
      (`self.Roam`))))

(event `self.HitBox.OnComponentBeginOverlap`
  (params (OverlappedComponent :type "PrimitiveComponent Object Reference") (OtherActor :type "Actor Object Reference") (OtherComp :type "PrimitiveComponent Object Reference") (OtherBodyIndex :type Integer) (bFromSweep :type Boolean) (SweepResult :type "HitResult Structure (by ref)"))
  ;[1 1 1] Hit player
  (bind _astorch_controller (cast `/Game/Blueprints/TorchController` OtherActor))
  (`KismetSystemLibrary.PrintString` "I AM HITTING YOU")
  (set `self.Attacking` true)
  (set `CharacterMovementComponent.MaxWalkSpeed` 0.0 (`self.CharacterMovement`))
  (`KismetSystemLibrary.Delay` 1.0)
  (if (`self.IsOverlappingActor` _astorch_controller)
    (`GameplayStatics.ApplyDamage` (`GameplayStatics.GetPlayerCharacter` 0) (`self.Damage`)))
  (`KismetSystemLibrary.Delay` 0.0)
  (set `self.Attacking` false)
  (`self.Chase`))

(event `self.PawnSensing.OnSeePawn`
  (params (Pawn :type "Pawn Object Reference"))
  ;[1 1 1] Trigger Chase
  (`self.Chase`))

(event `self.ReceiveTick`
  (params (DeltaSeconds :type "Float (single-precision)"))
  ;[1 1 1] Check Health
  (if (<= (`self.Health`) 0.0)
    (`KismetSystemLibrary.PrintString` "DED")
    (set `self.IsDead` true)
    (`self.K2_DestroyActor`)))

(event `self.InteractableArea.OnComponentBeginOverlap`
  (params (OverlappedComponent :type "PrimitiveComponent Object Reference") (OtherActor :type "Actor Object Reference") (OtherComp :type "PrimitiveComponent Object Reference") (OtherBodyIndex :type Integer) (bFromSweep :type Boolean) (SweepResult :type "HitResult Structure (by ref)"))
  ;[1 1 1] Begin/End Player Interaction
  (`self.EnableInput` (`GameplayStatics.GetPlayerController` 0)))

(event `self.InteractableArea.OnComponentEndOverlap`
  (params (OverlappedComponent :type "PrimitiveComponent Object Reference") (OtherActor :type "Actor Object Reference") (OtherComp :type "PrimitiveComponent Object Reference") (OtherBodyIndex :type Integer))
  ;[1 1 1] Begin/End Player Interaction
  (`self.DisableInput` (`GameplayStatics.GetPlayerController` 0)))

(event `self.ReceiveAnyDamage`
  (params (Damage :type "Float (single-precision)") (DamageType :type "DamageType Object Reference") (InstigatedBy :type "Controller Object Reference") (DamageCauser :type "Actor Object Reference"))
  ;[1 1 1] Check for Damage
  (set `self.Health` (- (`self.Health`) Damage)))

(fn `UserConstructionScript`)