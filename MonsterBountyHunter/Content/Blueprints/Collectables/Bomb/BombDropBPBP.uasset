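; Dropped bomb actor that explodes two seconds after spawning, then destroys itself with a scaled-up explosion particle effect.
; After the delay, it checks the actor from the BasicHit begin-overlap output and damages it if still overlapping.
; An actor also inside the CriticalHit volume takes a second equal hit.
; The overlap event runs no logic, so only that single referenced actor can be damaged.
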(event `self.ReceiveBeginPlay`
  (`KismetSystemLibrary.Delay` 2.0)
  (if (`self.IsOverlappingActor` (stale `self.Basic hit.OnComponentBeginOverlap` OtherActor))
    (`GameplayStatics.ApplyDamage` (stale `self.Basic hit.OnComponentBeginOverlap` OtherActor) 50.0)
    (if (`PrimitiveComponent.IsOverlappingActor` (`self.Critical Hit`) (stale `self.Basic hit.OnComponentBeginOverlap` OtherActor))
      (`GameplayStatics.ApplyDamage` (stale `self.Basic hit.OnComponentBeginOverlap` OtherActor) 50.0)))
  (`self.K2_DestroyActor`)
  (`GameplayStatics.SpawnEmitterAtLocation` "/Game/Art/StarterContent/Particles/P_Explosion.P_Explosion" (`self.K2_GetActorLocation`) (struct) (3.0 3.0 3.0)))

(event `self.Basic hit.OnComponentBeginOverlap`
  (params (OverlappedComponent :type "PrimitiveComponent Object Reference") (OtherActor :type "Actor Object Reference") (OtherComp :type "PrimitiveComponent Object Reference") (OtherBodyIndex :type Integer) (bFromSweep :type Boolean) (SweepResult :type "HitResult Structure (by ref)")))

(fn `UserConstructionScript`)