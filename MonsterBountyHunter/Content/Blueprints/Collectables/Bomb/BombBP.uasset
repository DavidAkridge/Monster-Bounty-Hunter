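; BombBP is a collectable pickup that adds bombs to the player's count.
; A timeline started on BeginPlay drives the yaw of its root component to rotate it.
; InteractableArea overlaps toggle input for player 0 without checking the overlapping actor, so Interact is gated by proximity.
; Pressing Interact increases Bombs on the TorchController player character, prints a string and destroys the pickup.
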(event `self.ReceiveBeginPlay`
  (bind (_direction _newtrack_0) (`Timeline|Rotation`)
    (:`Update`
      (`SceneComponent.K2_SetRelativeRotation` (`self.DefaultSceneRoot`) (`KismetMathLibrary.MakeRotator` 0.0 0.0 _newtrack_0) false false))))

(event `self.InteractableArea.OnComponentBeginOverlap`
  (params (OverlappedComponent :type "PrimitiveComponent Object Reference") (OtherActor :type "Actor Object Reference") (OtherComp :type "PrimitiveComponent Object Reference") (OtherBodyIndex :type Integer) (bFromSweep :type Boolean) (SweepResult :type "HitResult Structure (by ref)"))
  ;[1 1 1] Begin/End Player Interaction
  (`self.EnableInput` (`GameplayStatics.GetPlayerController` 0)))

(event `InputAction|Interact`
  (params (Key :type "Key Structure"))
  (:`Pressed`
    (bind _astorch_controller (cast `/Game/Blueprints/TorchController` (`GameplayStatics.GetPlayerCharacter` 0)))
    (set `/Game/Blueprints/TorchController.Bombs` (+ (`/Game/Blueprints/TorchController.Bombs` _astorch_controller) 3) _astorch_controller)
    (`KismetSystemLibrary.PrintString` (`KismetStringLibrary.Conv_IntToString` 0))
    (`self.K2_DestroyActor`)))

(event `self.InteractableArea.OnComponentEndOverlap`
  (params (OverlappedComponent :type "PrimitiveComponent Object Reference") (OtherActor :type "Actor Object Reference") (OtherComp :type "PrimitiveComponent Object Reference") (OtherBodyIndex :type Integer))
  ;[1 1 1] Begin/End Player Interaction
  (`self.DisableInput` (`GameplayStatics.GetPlayerController` 0)))

(fn `UserConstructionScript`)