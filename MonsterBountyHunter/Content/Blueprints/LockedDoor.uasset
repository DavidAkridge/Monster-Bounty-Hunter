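; Double door Blueprint that stays locked until its UnlockDoor event clears IsLocked.
; Overlapping InteractableArea enables player input, and leaving disables it, so Interact only works nearby.
; Interact prints a locked message or plays or reverses two timelines that set each door's yaw, with Door2 offset.
; A FlipFlop on the first timeline's finish sets IsOpen, which picks the next direction.
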(event `self.InteractableArea.OnComponentBeginOverlap`
  (params (OverlappedComponent :type "PrimitiveComponent Object Reference") (OtherActor :type "Actor Object Reference") (OtherComp :type "PrimitiveComponent Object Reference") (OtherBodyIndex :type Integer) (bFromSweep :type Boolean) (SweepResult :type "HitResult Structure (by ref)"))
  ;[1 1 1] Begin/End Player Interaction
  (`self.EnableInput` (`GameplayStatics.GetPlayerController` 0)))

(event `InputAction|Interact`
  (params (Key :type "Key Structure"))
  ;[1 1 1] InteractWitihDoor
  (:`Pressed`
    (if (`self.IsLocked`)
      (`KismetSystemLibrary.PrintString` "Door Locked!")
      (elif (`self.IsOpen`)
        (`|ExecutionSequence`
          (:`then_0`
            (bind (_direction _doorpos) (`Timeline|Door Open/Close` :!via `Reverse` :!label _label)
              (:`Update`
                (`SceneComponent.K2_SetRelativeRotation` (`self.Door1`) (`KismetMathLibrary.MakeRotator` 0.0 0.0 _doorpos) false false))
              (:`Finished`
                (`/Engine/EditorBlueprintResources/StandardMacros.FlipFlop`
                  (:`A`
                    (set `self.IsOpen` false))
                  (:`B`
                    (set `self.IsOpen` true))))))
          (:`then_1`
            (bind (_direction_2 _doorpos_2) (`Timeline|Door2 Open/Close` :!via `Reverse` :!label _label_2)
              (:`Update`
                (`SceneComponent.K2_SetRelativeRotation` (`self.Door2`) (`KismetMathLibrary.MakeRotator` 0.0 0.0 (- _doorpos_2 -80.0)) false false)))))
        (else
          (`|ExecutionSequence`
            (:`then_0`
              (goto _label))
            (:`then_1`
              (goto _label_2))))))))

(event `self.InteractableArea.OnComponentEndOverlap`
  (params (OverlappedComponent :type "PrimitiveComponent Object Reference") (OtherActor :type "Actor Object Reference") (OtherComp :type "PrimitiveComponent Object Reference") (OtherBodyIndex :type Integer))
  ;[1 1 1] Begin/End Player Interaction
  (`self.DisableInput` (`GameplayStatics.GetPlayerController` 0)))

(event `UnlockDoor`
  ;[1 1 1] Unlock Door
  (set `self.IsLocked` false))

(fn `UserConstructionScript`)