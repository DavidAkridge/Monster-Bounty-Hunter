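; Enemy actor that reacts to seeing a TorchController pawn by rotating and shooting.
; PawnSensing triggers a cast check, then a look-at rotation whose start and target both read GetActorLocation with no explicit target.
; It then spawns another TorchController as the projectile at ProjectileSpawnLocation and launches its mesh along the Cube's forward vector by ShootAmount.
; The SpawnProjectile flag and a short delay limit the fire rate.
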(event `self.PawnSensing.OnSeePawn`
  (params (Pawn :type "Pawn Object Reference"))
  ;[1 1 1] LookAndShoot
  (`KismetSystemLibrary.PrintString` "Hello")
  (cast `/Game/Blueprints/TorchController` Pawn)
  (`|ExecutionSequence`
    (:`then_0`
      (`self.K2_SetActorRotation` (`KismetMathLibrary.FindLookAtRotation` (`self.K2_GetActorLocation`) (`self.K2_GetActorLocation`))))
    (:`then_1`
      (if (`self.SpawnProjectile`)
        (bind _returnvalue (`|SpawnActorFromClass` "/Game/Blueprints/TorchController.TorchController_C" (`SceneComponent.K2_GetComponentToWorld` (`self.ProjectileSpawnLocation`)) "Undefined" "OverrideRootScale" null null))
        (`PrimitiveComponent.AddImpulse` (`Character.Mesh` _returnvalue) (* (`SceneComponent.GetForwardVector` (`self.Cube`)) (`self.ShootAmount`)) "None" true)
        (set `self.SpawnProjectile` false)
        (`KismetSystemLibrary.Delay` 0.2)
        (set `self.SpawnProjectile` true)))))

(fn `UserConstructionScript`)