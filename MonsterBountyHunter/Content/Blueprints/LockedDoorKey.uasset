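; LockedDoorKey is a pickup key actor that unlocks a linked locked door when the player interacts with it.
; Overlapping its InteractableArea enables input for player controller 0, and ending the overlap disables it.
; Pressing Interact loops over the LockedDoor array, but only acts when the array holds a single entry.
; It then calls UnlockDoor on that door, destroys the key and prints a confirmation message.
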(event `self.InteractableArea.OnComponentBeginOverlap`
  (params (OverlappedComponent :type "PrimitiveComponent Object Reference") (OtherActor :type "Actor Object Reference") (OtherComp :type "PrimitiveComponent Object Reference") (OtherBodyIndex :type Integer) (bFromSweep :type Boolean) (SweepResult :type "HitResult Structure (by ref)"))
  ;[1 1 1] Begin/End Player Interaction
  (`self.EnableInput` (`GameplayStatics.GetPlayerController` 0)))

(event `InputAction|Interact`
  (params (Key :type "Key Structure"))
  (bind _lockeddoor (`self.LockedDoor`))
  (:`Pressed`
    (for _array_element _lockeddoor
      (if (< (`KismetArrayLibrary.Array_LastIndex` _lockeddoor) 1)
        (`/Game/Blueprints/LockedDoor.UnlockDoor` _array_element)
        (`self.K2_DestroyActor`)
        (`KismetSystemLibrary.PrintString` "Key Obtained!")))))

(event `self.InteractableArea.OnComponentEndOverlap`
  (params (OverlappedComponent :type "PrimitiveComponent Object Reference") (OtherActor :type "Actor Object Reference") (OtherComp :type "PrimitiveComponent Object Reference") (OtherBodyIndex :type Integer))
  ;[1 1 1] Begin/End Player Interaction
  (`self.DisableInput` (`GameplayStatics.GetPlayerController` 0)))

(fn `UserConstructionScript`)