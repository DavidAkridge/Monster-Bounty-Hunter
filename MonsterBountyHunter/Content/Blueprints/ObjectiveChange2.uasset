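; An overlap trigger actor that advances the player's objective to Objective2 and saves that progress.
; When a TorchController overlaps it, the controller's PlayerObjective is set directly.
; It then loads the MonsterSaveGame slot, or creates a new save object if none exists, writes the same objective into it and saves.
; The save result is printed to screen as debug output.
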(event `self.ReceiveActorBeginOverlap`
  (params (OtherActor :type "Actor Object Reference"))
  (bind _saversubclass (`self.SaverSubClass`))
  (bind _astorch_controller (cast `/Game/Blueprints/TorchController` OtherActor))
  (set `/Game/Blueprints/TorchController.PlayerObjective` "Objective2" _astorch_controller)
  (bind _returnvalue (`GameplayStatics.DoesSaveGameExist` "MonsterSaveGame"))
  (if _returnvalue
    (bind _returnvalue_2 (`GameplayStatics.LoadGameFromSlot` "MonsterSaveGame"))
    (bind _output_get (set `self.SaverSubClass` _returnvalue_2))
    (bind _asmonster_save_game (cast `/Game/Blueprints/MonsterSaveGame` _output_get))
    (set `/Game/Blueprints/MonsterSaveGame.PlayerObjective` "Objective2" _asmonster_save_game)
    (bind _returnvalue_3 (`GameplayStatics.SaveGameToSlot` _saversubclass "MonsterSaveGame"))
    (`KismetSystemLibrary.PrintString` (`KismetStringLibrary.Conv_BoolToString` _returnvalue_3))
    (else
      (bind _returnvalue_4 (`GameplayStatics.CreateSaveGameObject` "/Game/Blueprints/MonsterSaveGame.MonsterSaveGame_C"))
      (bind _output_get_2 (set `self.SaverSubClass` _returnvalue_4))
      (bind _asmonster_save_game_2 (cast `/Game/Blueprints/MonsterSaveGame` _output_get_2))
      (set `/Game/Blueprints/MonsterSaveGame.PlayerObjective` "Objective2" _asmonster_save_game_2)
      (bind _returnvalue_5 (`GameplayStatics.SaveGameToSlot` _saversubclass "MonsterSaveGame"))
      (`KismetSystemLibrary.PrintString` (`KismetStringLibrary.Conv_BoolToString` _returnvalue_5)))))

(fn `UserConstructionScript`)